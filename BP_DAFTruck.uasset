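; DAF truck Blueprint for the Carla simulator, with scaffolding for spotlight control and trailer coupling.
; BeginPlay caches its SpotLight components and calls ToggleLight, which only prints a debug string because the visibility loop is unwired.
; A function spawns BP_Trailer at a mesh socket transform (socket name None), but is never called.
; Coupling is left to a Python script, as Carla does not see a Blueprint-spawned trailer.
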(event `self.ReceiveBeginPlay`
  (bind _output_get (set `self.LightsArray` (`self.K2_GetComponentsByClass` "/Script/Engine.SpotLightComponent")))
  (`self.ToggleLight` true))

(event `ToggleLight`
  (params (LightState :type Boolean))
  (`KismetSystemLibrary.PrintString` "ToggleLight 실행됨!ToggleLight 실행됨!"))

(fn `Couple the trailer at begin play`
  (`|SpawnActorFromClass` "/Game/Carla/Blueprints/Vehicles/Trailer/BP_Trailer.BP_Trailer_C" (`KismetMathLibrary.MakeTransform` (`SceneComponent.GetSocketLocation` (`self.Mesh`) "None") (`SceneComponent.GetSocketRotation` (`self.Mesh`) "None")) "AlwaysSpawn" "OverrideRootScale" null null null))

(fn `UserConstructionScript`
  (`parent.UserConstructionScript`))